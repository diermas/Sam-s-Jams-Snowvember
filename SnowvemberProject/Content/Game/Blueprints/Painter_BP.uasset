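; Painter actor that marks the player as paintable while the player overlaps it.
; Begin and end overlap events check that the other actor's class is exactly Player_BP, then set its Paintable flag on or off.
; The flag is written to the instance returned by GetActorOfClass rather than to the overlapping actor, which effectively assumes a single player.
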(event `self.ReceiveActorBeginOverlap`
  (params (OtherActor :type "Actor Object Reference"))
  (if (== (`GameplayStatics.GetObjectClass` OtherActor) "/Game/Game/Blueprints/Player_BP.Player_BP_C")
    (bind _returnvalue (`GameplayStatics.GetActorOfClass` "/Game/Game/Blueprints/Player_BP.Player_BP_C"))
    (set `/Game/Game/Blueprints/Player_BP.Paintable` true _returnvalue)))

(event `self.ReceiveActorEndOverlap`
  (params (OtherActor :type "Actor Object Reference"))
  (if (== (`GameplayStatics.GetObjectClass` OtherActor) "/Game/Game/Blueprints/Player_BP.Player_BP_C")
    (bind _returnvalue (`GameplayStatics.GetActorOfClass` "/Game/Game/Blueprints/Player_BP.Player_BP_C"))
    (set `/Game/Game/Blueprints/Player_BP.Paintable` false _returnvalue)))

(fn `UserConstructionScript`)