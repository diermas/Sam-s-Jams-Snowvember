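; A moving platform that travels in X and Z and is passable or solid depending on the player's colour.
; At BeginPlay it caches start and end positions, then a timeline scaled by Speed lerps it between them with a swept move, holding Y fixed.
; On any actor overlap it looks up Player_BP and switches Collision to NoCollision if the colours match, otherwise BlockAll.
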(event `self.ReceiveBeginPlay`
  (bind (_returnvalue_x _returnvalue_y _returnvalue_z) (`KismetMathLibrary.BreakVector` (`self.K2_GetActorLocation`)))
  (`TimelineComponent.SetPlayRate` (`self.LerpTimeline`) (`self.Speed`))
  (set `self.YPos` _returnvalue_y)
  (bind _output_get (set `self.StartX` _returnvalue_x))
  (bind _output_get_2 (set `self.StartZ` _returnvalue_z))
  (set `self.EndX` (+ _output_get (`self.DistanceX`)))
  (set `self.EndZ` (+ _output_get_2 (`self.DistanceZ`)))
  (bind (_direction _value) (`Timeline|LerpTimeline` :`NewTime` 0.0)
    (:`Update`
      (`self.K2_SetActorLocation` (`KismetMathLibrary.MakeVector` (`KismetMathLibrary.Lerp` (`self.StartX`) (`self.EndX`) _value) (`self.YPos`) (`KismetMathLibrary.Lerp` (`self.StartZ`) (`self.EndZ`) _value)) true))))

(event `self.ReceiveActorBeginOverlap`
  (params (OtherActor :type "Actor Object Reference"))
  (bind _collision (`self.Collision`))
  (bind _returnvalue (`GameplayStatics.GetActorOfClass` "/Game/Game/Blueprints/Player_BP.Player_BP_C"))
  (if (== (`/Game/Game/Blueprints/Player_BP.Colour` _returnvalue) (`self.Colour`))
    (`PrimitiveComponent.SetCollisionProfileName` _collision "NoCollision")
    (else
      (`PrimitiveComponent.SetCollisionProfileName` _collision "BlockAll"))))

(fn `UserConstructionScript`)