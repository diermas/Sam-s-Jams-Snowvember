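; Player pawn with a flipbook sprite that moves left and right along X and can switch between red, blue, green and yellow.
; Number keys swap colour while Paintable is true, storing the colour name and carrying playback position across flipbooks so animation stays in step.
; Movement plays the flipbook forward or reversed by direction, and Tick stops it when velocity is zero.
; Enter opens the main menu level and Escape quits the game.
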(event `Key|One`
  (params (Key :type "Key Structure"))
  (bind _sprite (`self.Sprite`))
  (:`Released`
    (if (`self.Paintable`)
      (set `self.Colour` "Red")
      (bind _output_get (set `self.CurrentFrame` (`PaperFlipbookComponent.GetPlaybackPosition` _sprite)))
      (`PaperFlipbookComponent.SetFlipbook` _sprite "/Game/Game/Sprites/RedFlipbook.RedFlipbook")
      (`PaperFlipbookComponent.SetPlaybackPosition` _sprite _output_get false))))

(event `Key|Two`
  (params (Key :type "Key Structure"))
  (bind _sprite (`self.Sprite`))
  (:`Released`
    (if (`self.Paintable`)
      (set `self.Colour` "Blue")
      (bind _output_get (set `self.CurrentFrame` (`PaperFlipbookComponent.GetPlaybackPosition` _sprite)))
      (`PaperFlipbookComponent.SetFlipbook` _sprite "/Game/Game/Sprites/BlueFlipbook.BlueFlipbook")
      (`PaperFlipbookComponent.SetPlaybackPosition` _sprite _output_get false))))

(event `Key|Three`
  (params (Key :type "Key Structure"))
  (bind _sprite (`self.Sprite`))
  (:`Released`
    (if (`self.Paintable`)
      (set `self.Colour` "Green")
      (bind _output_get (set `self.CurrentFrame` (`PaperFlipbookComponent.GetPlaybackPosition` _sprite)))
      (`PaperFlipbookComponent.SetFlipbook` _sprite "/Game/Game/Sprites/GreenFlipbook.GreenFlipbook")
      (`PaperFlipbookComponent.SetPlaybackPosition` _sprite _output_get false))))

(event `Key|Four`
  (params (Key :type "Key Structure"))
  (bind _sprite (`self.Sprite`))
  (:`Released`
    (if (`self.Paintable`)
      (set `self.Colour` "Yellow")
      (bind _output_get (set `self.CurrentFrame` (`PaperFlipbookComponent.GetPlaybackPosition` _sprite)))
      (`PaperFlipbookComponent.SetFlipbook` _sprite "/Game/Game/Sprites/YellowFlipbook.YellowFlipbook")
      (`PaperFlipbookComponent.SetPlaybackPosition` _sprite _output_get false))))

(event `self.ReceiveTick`
  (params (DeltaSeconds :type "Float (single-precision)"))
  ;[1 1 1] Pause the animation when character is still
  (if (not (!= (`self.GetVelocity`) (0.0 0.0 0.0)))
    (`PaperFlipbookComponent.Stop` (`self.Sprite`))))

(event `InputAxis|MoveRight`
  (params (AxisValue :type "Float (single-precision)"))
  (bind _sprite (`self.Sprite`))
  ;[1 1 1] Movement controls for left and right, and update animation direction
  (if (!= AxisValue 0.0)
    (if (> AxisValue 0.0)
      (`self.AddMovementInput` (1.0 0.0 0.0))
      (`PaperFlipbookComponent.Play` _sprite)
      (else
        (`self.AddMovementInput` (-1.0 0.0 0.0))
        (`PaperFlipbookComponent.Reverse` _sprite)))))

(event `Key|Enter`
  (params (Key :type "Key Structure"))
  (:`Released`
    (`GameplayStatics.OpenLevel` "MainMenuLevel")))

(event `Key|Escape`
  (params (Key :type "Key Structure"))
  (:`Released`
    (`KismetSystemLibrary.QuitGame` null "Quit")))

(fn `UserConstructionScript`)